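; BP_Door is a Level 2 door trigger that plays a camera move and relocates the 2D player when its Box is overlapped.
; The overlap, with no check on the other actor, disables input on BP_PlayerController2D while a timeline slides the BP_Player2d_1 camera along negative Y.
; On finish, it moves the player to a hard-coded location, snaps the camera to the player's mesh position and restores input.
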(event `self.Box.OnComponentBeginOverlap`
  (params (OverlappedComponent :type "PrimitiveComponent Object Reference") (OtherActor :type "Actor Object Reference") (OtherComp :type "PrimitiveComponent Object Reference") (OtherBodyIndex :type Integer) (bFromSweep :type Boolean) (SweepResult :type "HitResult Structure (by ref)"))
  (bind _returnvalue (`GameplayStatics.GetActorOfClass` "/Game/Blueprint/Character/BP_PlayerController2D.BP_PlayerController2D_C"))
  (`self.DisableInput` _returnvalue null)
  (bind _returnvalue_2 (`GameplayStatics.GetActorOfClass` "/Game/Blueprint/Character/BP_Player2d_1.BP_Player2d_1_C"))
  (bind _camera (`/Game/Blueprint/Character/BP_Player2d_1.Camera` _returnvalue_2))
  (bind _output_get (set `self.Origin` (`SceneComponent.K2_GetComponentLocation` _camera)))
  (bind (_direction _pista_nueva_0) (`Timeline|Cronograma` :!via `PlayFromStart`)
    (:`Update`
      (`SceneComponent.K2_SetWorldLocation` _camera (`KismetMathLibrary.MakeVector` (.x _output_get) (- (.y _output_get) (* _pista_nueva_0 125.0)) (.z _output_get)) false false))
    (:`Finished`
      (`SceneComponent.K2_SetWorldLocation` (`Actor.RootComponent` _returnvalue_2) (22.0 0.0 47.0) false false)
      (bind _returnvalue_location (`KismetMathLibrary.BreakTransform` (`SceneComponent.K2_GetComponentToWorld` (`Character.Mesh` _returnvalue_2))))
      (`SceneComponent.K2_SetWorldLocation` _camera _returnvalue_location false false)
      (`self.EnableInput` _returnvalue null))))

(fn `UserConstructionScript`)