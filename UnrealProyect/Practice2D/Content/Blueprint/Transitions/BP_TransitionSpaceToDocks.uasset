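; Level transition trigger that takes the 2D player to Level_Docks when they overlap BoxLeft.
; Overlap flags a cutscene, disables input, fades the camera to black and removes all widgets.
; StartTransition timeline nudges the player along +X and the spring arm along -X each update, using incremental offsets.
; A second timeline then drives Room_1's MainMusic volume before a short delay, clearing the flag and opening the level.
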(event `self.BoxLeft.OnComponentBeginOverlap`
  (params (OverlappedComponent :type "PrimitiveComponent Object Reference") (OtherActor :type "Actor Object Reference") (OtherComp :type "PrimitiveComponent Object Reference") (OtherBodyIndex :type Integer) (bFromSweep :type Boolean) (SweepResult :type "HitResult Structure (by ref)"))
  (bind _asbp_player_2d_1 (cast `/Game/Blueprint/Character/BP_Player2d_1` OtherActor))
  (set `/Game/Blueprint/Character/BP_Player2d_1.bIsCutscene` true _asbp_player_2d_1)
  (`PrimitiveComponent.SetCollisionEnabled` (`Character.CapsuleComponent` _asbp_player_2d_1) "QueryAndPhysics")
  (bind _playercontroller (`/Game/Blueprint/Character/BP_Player2d_1.PlayerController` _asbp_player_2d_1))
  (`self.DisableInput` _playercontroller _playercontroller)
  (`PlayerCameraManager.StartCameraFade` (`PlayerController.PlayerCameraManager` _playercontroller) 0.0 1.0 1.0 (struct :`A` 1.0) false true)
  (`WidgetLayoutLibrary.RemoveAllWidgets`)
  (bind (_direction _alpha) (`Timeline|StartTransition` :!via `PlayFromStart`)
    (:`Update`
      (bind _springarm (`/Game/Blueprint/Character/BP_Player2d_1.SpringArm` _asbp_player_2d_1))
      (`SceneComponent.K2_SetRelativeLocation` _springarm (+ (`SceneComponent.RelativeLocation` _springarm) (`KismetMathLibrary.MakeVector` (* _alpha -10.0))) false false)
      (`self.K2_SetActorLocation` _asbp_player_2d_1 (+ (`self.K2_GetActorLocation` _asbp_player_2d_1) (`KismetMathLibrary.MakeVector` (* _alpha 3.0))) false false))
    (:`Finished`
      (bind _returnvalue (`GameplayStatics.GetActorOfClass` "/Game/Blueprint/Level_2_Rooms/Room_1.Room_1_C"))
      (bind (_direction_2 _a) (`Timeline|Timeline` :!via `PlayFromStart`)
        (:`Update`
          (`AudioComponent.SetVolumeMultiplier` (`/Game/Blueprint/Level_2_Rooms/Room_1.MainMusic` _returnvalue) _a))
        (:`Finished`
          (`KismetSystemLibrary.Delay` 0.5)
          (set `/Game/Blueprint/Character/BP_Player2d_1.bIsCutscene` false _asbp_player_2d_1)
          (`GameplayStatics.OpenLevel` "Level_Docks"))))))

(fn `UserConstructionScript`)