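; Two-way screen transition for BP_Player2d_1, triggered by overlapping either the left or right box.
; Each box flags a cutscene, disables input and fades to black while a timeline nudges the player along X and slides the spring arm oppositely.
; After a short delay it clears the flag and fades in, as a second timeline reverses the camera slide and pins the player at that side's destination arrow, then restores input.
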(event `self.BoxLeft.OnComponentBeginOverlap`
  (params (OverlappedComponent :type "PrimitiveComponent Object Reference") (OtherActor :type "Actor Object Reference") (OtherComp :type "PrimitiveComponent Object Reference") (OtherBodyIndex :type Integer) (bFromSweep :type Boolean) (SweepResult :type "HitResult Structure (by ref)"))
  (bind _asbp_player_2d_1 (cast `/Game/Blueprint/Character/BP_Player2d_1` OtherActor))
  (set `/Game/Blueprint/Character/BP_Player2d_1.bIsCutscene` true _asbp_player_2d_1)
  (`PrimitiveComponent.SetCollisionEnabled` (`Character.CapsuleComponent` _asbp_player_2d_1) "QueryAndPhysics")
  (bind _playercontroller (`/Game/Blueprint/Character/BP_Player2d_1.PlayerController` _asbp_player_2d_1))
  (`self.DisableInput` _playercontroller _playercontroller)
  (bind _playercameramanager (`PlayerController.PlayerCameraManager` _playercontroller))
  (`PlayerCameraManager.StartCameraFade` _playercameramanager 0.0 1.0 1.0 (struct :`A` 1.0) false true)
  (bind (_direction _alpha) (`Timeline|StartTransition` :!via `PlayFromStart`)
    (:`Update`
      (bind _springarm (`/Game/Blueprint/Character/BP_Player2d_1.SpringArm` _asbp_player_2d_1))
      (`SceneComponent.K2_SetRelativeLocation` _springarm (+ (`SceneComponent.RelativeLocation` _springarm) (`KismetMathLibrary.MakeVector` (* _alpha -10.0))) false false)
      (`self.K2_SetActorLocation` _asbp_player_2d_1 (+ (`self.K2_GetActorLocation` _asbp_player_2d_1) (`KismetMathLibrary.MakeVector` (* _alpha 3.0))) false false))
    (:`Finished`
      (`KismetSystemLibrary.Delay` 0.5)
      (set `/Game/Blueprint/Character/BP_Player2d_1.bIsCutscene` false _asbp_player_2d_1)
      (`PlayerCameraManager.StartCameraFade` _playercameramanager 1.0 0.0 1.0 (struct :`A` 1.0) false false)
      (bind (_direction_2 _alpha_2) (`Timeline|EndTransition` :!via `PlayFromStart`)
        (:`Update`
          (`SceneComponent.K2_SetRelativeLocation` _springarm (+ (`SceneComponent.RelativeLocation` _springarm) (`KismetMathLibrary.MakeVector` (* _alpha_2 10.0))) false false)
          (`self.K2_SetActorLocation` _asbp_player_2d_1 (`SceneComponent.K2_GetComponentLocation` (`self.Arrow1`)) false false))
        (:`Finished`
          (`self.EnableInput` _playercontroller _playercontroller)
          (`PrimitiveComponent.SetCollisionEnabled` (`Character.CapsuleComponent` _asbp_player_2d_1) "QueryAndPhysics"))))))

(event `self.BoxRight.OnComponentBeginOverlap`
  (params (OverlappedComponent :type "PrimitiveComponent Object Reference") (OtherActor :type "Actor Object Reference") (OtherComp :type "PrimitiveComponent Object Reference") (OtherBodyIndex :type Integer) (bFromSweep :type Boolean) (SweepResult :type "HitResult Structure (by ref)"))
  (bind _asbp_player_2d_1 (cast `/Game/Blueprint/Character/BP_Player2d_1` OtherActor))
  (set `/Game/Blueprint/Character/BP_Player2d_1.bIsCutscene` true _asbp_player_2d_1)
  (`PrimitiveComponent.SetCollisionEnabled` (`Character.CapsuleComponent` _asbp_player_2d_1) "QueryAndPhysics")
  (bind _playercontroller (`/Game/Blueprint/Character/BP_Player2d_1.PlayerController` _asbp_player_2d_1))
  (`self.DisableInput` _playercontroller _playercontroller)
  (bind _playercameramanager (`PlayerController.PlayerCameraManager` _playercontroller))
  (`PlayerCameraManager.StartCameraFade` _playercameramanager 0.0 1.0 1.0 (struct :`A` 1.0) false true)
  (bind (_direction _alpha) (`Timeline|Timeline` :!via `PlayFromStart`)
    (:`Update`
      (bind _springarm (`/Game/Blueprint/Character/BP_Player2d_1.SpringArm` _asbp_player_2d_1))
      (`SceneComponent.K2_SetRelativeLocation` _springarm (+ (`SceneComponent.RelativeLocation` _springarm) (`KismetMathLibrary.MakeVector` (* _alpha 10.0))) false false)
      (`self.K2_SetActorLocation` _asbp_player_2d_1 (+ (`self.K2_GetActorLocation` _asbp_player_2d_1) (`KismetMathLibrary.MakeVector` (* _alpha -3.0))) false false))
    (:`Finished`
      (`KismetSystemLibrary.Delay` 0.5)
      (set `/Game/Blueprint/Character/BP_Player2d_1.bIsCutscene` false _asbp_player_2d_1)
      (`PlayerCameraManager.StartCameraFade` _playercameramanager 1.0 0.0 1.0 (struct :`A` 1.0) false false)
      (bind (_direction_2 _alpha_2) (`Timeline|Timeline_0` :!via `PlayFromStart`)
        (:`Update`
          (`SceneComponent.K2_SetRelativeLocation` _springarm (+ (`SceneComponent.RelativeLocation` _springarm) (`KismetMathLibrary.MakeVector` (* _alpha_2 -10.0))) false false)
          (`self.K2_SetActorLocation` _asbp_player_2d_1 (`SceneComponent.K2_GetComponentLocation` (`self.Arrow`)) false false))
        (:`Finished`
          (`self.EnableInput` _playercontroller _playercontroller)
          (`PrimitiveComponent.SetCollisionEnabled` (`Character.CapsuleComponent` _asbp_player_2d_1) "QueryAndPhysics"))))))

(fn `UserConstructionScript`)