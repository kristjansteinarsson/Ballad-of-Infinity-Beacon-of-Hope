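; Short-lived light melee attack actor that displays a slash sprite and manages its owning player's attack state.
; Generate picks the sprite from the combo value; the weapon type switch has only a default branch.
; It flags the controller as attacking, lowers gravity and calls StopRN on a falling player.
; After a brief delay it restores gravity, calls Attacking on the player, clears the flag and destroys itself.
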(event `Generate`
  (bind _playerowner (`self.PlayerOwner`))
  (bind _playerowner_2 (`self.PlayerOwner`))
  (bind _charactermovement (`Character.CharacterMovement` _playerowner_2))
  (bind _playercontroller (`/Game/Blueprint/Character/BP_Player2d_1.PlayerController` _playerowner_2))
  (switch `int` (`self.WeaponType`)
    (:`Default`
      (switch `int` (`self.ComboValue`)
        (:`Default`
          (`PaperSpriteComponent.SetSprite` (`self.PaperSprite`) "/Game/OurAssets/MeleeAttacks/Slashes_Sprite_sheet_Sprite_0.Slashes_Sprite_sheet_Sprite_0"))
        (:`1`
          (`PaperSpriteComponent.SetSprite` (`self.PaperSprite`) "/Game/OurAssets/MeleeAttacks/Slashes_Sprite_sheet_Sprite_1.Slashes_Sprite_sheet_Sprite_1"))
        (:`2`
          (`PaperSpriteComponent.SetSprite` (`self.PaperSprite`) "/Game/OurAssets/MeleeAttacks/Slashes_Sprite_sheet_Sprite_2.Slashes_Sprite_sheet_Sprite_2"))
        (:`3`
          (`PaperSpriteComponent.SetSprite` (`self.PaperSprite`) "/Game/OurAssets/MeleeAttacks/Slashes_Sprite_sheet_Sprite_3.Slashes_Sprite_sheet_Sprite_3"))
        (:`4`
          (`PaperSpriteComponent.SetSprite` (`self.PaperSprite`) "/Game/OurAssets/MeleeAttacks/Slashes_Sprite_sheet_Sprite_4.Slashes_Sprite_sheet_Sprite_4")))
      (set `/Game/Blueprint/Character/BP_PlayerController2D.IsCharacterAttacking` true _playercontroller)
      (set `CharacterMovementComponent.GravityScale` 0.4 _charactermovement)
      (if (`NavMovementInterface.IsFalling` _charactermovement)
        (`/Game/Blueprint/Character/BP_Player2d_1.StopRN` _playerowner))
      (`KismetSystemLibrary.Delay` 0.4)
      (set `CharacterMovementComponent.GravityScale` 1.0 (`Character.CharacterMovement` _playerowner))
      (`/Game/Blueprint/Character/BP_Player2d_1.Attacking` _playerowner)
      (set `/Game/Blueprint/Character/BP_PlayerController2D.IsCharacterAttacking` false _playercontroller)
      (`self.K2_DestroyActor`))))

(fn `UserConstructionScript`)