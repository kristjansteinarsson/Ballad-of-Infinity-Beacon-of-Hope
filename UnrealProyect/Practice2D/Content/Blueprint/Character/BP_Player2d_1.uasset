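; 2D player character with movement, combo attacks, dodge rolls, coin pickup, damage and death that reloads the level.
; Tick picks flipbooks from movement state, and facing mirrors the sprite via X scale.
; Attack spawns an attached attack actor with data-table damage and a combo count, which a self-looping delay timer resets.
; Duplicate Roll macros loop timed impulses, disabling the hurtbox for i-frames.
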(event `self.ReceiveBeginPlay`
  (`self.ComboDecayTick`))

(event `ComboDecayTick`
  (if (> (`self.ComboDecay`) 0.0)
    (`KismetSystemLibrary.Delay` 0.1)
    (set `self.ComboDecay` (+ (`self.ComboDecay`) -0.1))
    (else
      (set `self.ComboValue` 0)
      (`KismetSystemLibrary.Delay` 0.1)))
  (`self.ComboDecayTick`))

(event `self.ReceiveTick`
  (params (DeltaSeconds :type "Float (single-precision)"))
  (bind _returnvalue_x (`KismetMathLibrary.BreakVector` (`self.GetVelocity`)))
  (bind (_returnvalue_x_2 _returnvalue_y _returnvalue_z) (`KismetMathLibrary.BreakVector` (`self.GetVelocity`)))
  (if (`self.bIsCutscene`)
    (`PaperFlipbookComponent.SetFlipbook` (`self.Flipbook`) "/Game/Craftpix/1_Main_Characters/1/FB_Double_Jump.FB_Double_Jump")
    (elif (`self.IsNotDead`)
      (if (`NavMovementComponent.IsMovingOnGround` (`self.CharacterMovement`))
        ;[0.05098 0.05098 0.05098] Decide between Idle or Run animation when grounded
        (`PaperFlipbookComponent.SetFlipbook` (`self.Flipbook`) (select `bool` (== _returnvalue_x 0.0) :`false` (`self.WalkSprite`) :`true` (`self.IdleSprite`)))
        (else
          ;[0.05098 0.05098 0.05098] Decide between JumpRise or Fall animation when airborne
          (`PaperFlipbookComponent.SetFlipbook` (`self.Flipbook`) (select `bool` (< _returnvalue_z 0.0) :`false` (`self.JumpSprite`) :`true` (`self.FallSprite`))))))))

(event `Death`
  (bind _flipbook (`self.Flipbook`))
  (`GameplayStatics.PlaySound2D` "/Engine/VREditor/Sounds/VR_negative.VR_negative" 1.0 1.0 0.0 null null)
  (`CharacterMovementComponent.DisableMovement` (`self.CharacterMovement`))
  (set `self.IsNotDead` false)
  (`PaperFlipbookComponent.SetFlipbook` _flipbook "/Game/Craftpix/1_Main_Characters/1/FB_Hit.FB_Hit")
  (`KismetSystemLibrary.Delay` (`PaperFlipbookComponent.GetFlipbookLength` _flipbook))
  (`self.MapReload`))

(event `MapReload`
  (bind _returnvalue (`GameplayStatics.GetCurrentLevelName` true))
  (`GameplayStatics.OpenLevel` (`KismetStringLibrary.Conv_StringToName` _returnvalue)))

(event `DodgeRoll`
  (bind _returnvalue (`|GetInputActionValue`))
  (if (!= _returnvalue 0.0)
    (if (> _returnvalue 0.0)
      (`PrimitiveComponent.SetCollisionEnabled` (`self.PlayerHurtBox`) "NoCollision" :!label _label)
      (if (and (!= (`self.RollDuration`) (`self.RollCount`)) (`NavMovementInterface.IsMovingOnGround` (`self.CharacterMovement`))) :!label _label_2
        (if (> (`self.RollCount`) (`self.RollIFrames`))
          (`PrimitiveComponent.SetCollisionEnabled` (`self.PlayerHurtBox`) "QueryAndPhysics"))
        (`CharacterMovementComponent.AddImpulse` (`self.CharacterMovement`) (* 1 (`KismetMathLibrary.MakeVector` 250.0)) true)
        (`KismetSystemLibrary.Delay` 0.03)
        (set `self.RollCount` (+ (`self.RollCount`) 1))
        (goto _label_2)
        (else
          (set `self.RollCount` 0)
          (`PrimitiveComponent.SetCollisionEnabled` (`self.PlayerHurtBox`) "QueryAndPhysics")))
      (else
        (`PrimitiveComponent.SetCollisionEnabled` (`self.PlayerHurtBox`) "NoCollision" :!label _label_3)
        (if (and (!= (`self.RollDuration`) (`self.RollCount`)) (`NavMovementInterface.IsMovingOnGround` (`self.CharacterMovement`))) :!label _label_4
          (if (> (`self.RollCount`) (`self.RollIFrames`))
            (`PrimitiveComponent.SetCollisionEnabled` (`self.PlayerHurtBox`) "QueryAndPhysics"))
          (`CharacterMovementComponent.AddImpulse` (`self.CharacterMovement`) (* -1 (`KismetMathLibrary.MakeVector` 250.0)) true)
          (`KismetSystemLibrary.Delay` 0.03)
          (set `self.RollCount` (+ (`self.RollCount`) 1))
          (goto _label_4)
          (else
            (set `self.RollCount` 0)
            (`PrimitiveComponent.SetCollisionEnabled` (`self.PlayerHurtBox`) "QueryAndPhysics")))))
    (else
      (switch `/Game/Blueprint/Character/LeftRightGame` (`self.LeftRight`)
        (:`NewEnumerator0`
          (goto _label_3))
        (:`NewEnumerator1`
          (goto _label))))))

(event `GetHit`
  (params (NewParam :type "/Game/Blueprint/Components/Str_Damage Structure"))
  (bind _takendamage (`/Game/Blueprint/Components/BP_Health.TakeDamage` (`self.BP_Health`) NewParam))
  (if (> _takendamage 0.0)
    _))

(fn `AddCoin`
  (params (Value :type Integer))
  (set `self.CurrentCoins` (+ (`self.CurrentCoins`) Value))
  (`GameplayStatics.PlaySound2D` "/Engine/VREditor/Sounds/VR_click3.VR_click3" 1.0 1.0 0.0 null null))

(fn `Attack`
  (locals (AttackInstance :type "/Game/Blueprint/Character/Attacks/Melee/BP_Attack_Light_1 Object Reference"))
  (bind _combovalue (`self.ComboValue`))
  (bind _attackinstance (`local.AttackInstance`))
  (if (>= (`self.ComboValue`) 5)
    (set `self.ComboValue` 0))
  (switch `/Game/Blueprint/Character/LeftRightGame` (`self.LeftRight`)
    (:`NewEnumerator0`
      (bind _returnvalue (`|SpawnActorFromClass` "/Game/Blueprint/Character/Attacks/Melee/BP_Attack_Light_1.BP_Attack_Light_1_C" (`KismetMathLibrary.MakeTransform` (-160.0 0.0 0.0) (struct) (`KismetMathLibrary.MakeVector` (.x (`SceneComponent.RelativeScale3D` (`self.Flipbook`))) (.y (`SceneComponent.RelativeScale3D` (`self.Flipbook`))) (.z (`SceneComponent.RelativeScale3D` (`self.Flipbook`))))) "Undefined" "MultiplyWithRoot" null null))
      (set `local.AttackInstance` _returnvalue))
    (:`NewEnumerator1`
      (bind _returnvalue_2 (`|SpawnActorFromClass` "/Game/Blueprint/Character/Attacks/Melee/BP_Attack_Light_1.BP_Attack_Light_1_C" (`KismetMathLibrary.MakeTransform` (160.0 0.0 0.0) (struct) (`KismetMathLibrary.MakeVector` (.x (`SceneComponent.RelativeScale3D` (`self.Flipbook`))) (.y (`SceneComponent.RelativeScale3D` (`self.Flipbook`))) (.z (`SceneComponent.RelativeScale3D` (`self.Flipbook`))))) "Undefined" "MultiplyWithRoot" null null))
      (set `local.AttackInstance` _returnvalue_2)))
  (set `/Game/Blueprint/Character/Attacks/Melee/BP_Attack_Light_1.WeaponType` 0 _attackinstance)
  (bind _returnvalue_3 (`|GetDataTableRow` (`self.WeaponDatatable`) (`self.WeaponRightHand`))
    (:`then`
      (set `/Game/Blueprint/Character/Attacks/Melee/BP_Attack_Light_1.Damage` (`.Damage_9_ED2352264D71B5BE100C1A96F9083D4C` (break `/Game/Blueprint/Character/Attacks/STR_MeleeWeapon` _returnvalue_3)) _attackinstance)
      (set `/Game/Blueprint/Character/Attacks/Melee/BP_Attack_Light_1.ComboValue` _combovalue _attackinstance)
      (set `self.ComboValue` (+ _combovalue 1))
      (set `/Game/Blueprint/Character/Attacks/Melee/BP_Attack_Light_1.PlayerOwner` self _attackinstance)
      (`/Game/Blueprint/Character/Attacks/Melee/BP_Attack_Light_1.Generate` _attackinstance)
      (`self.K2_AttachToActor` _attackinstance self "None" "KeepRelative" "KeepWorld" "KeepRelative" true)
      (set `self.ComboDecay` 0.5))))

(fn `FlipFunction`
  (bind _flipbook (`self.Flipbook`))
  (switch `/Game/Blueprint/Character/LeftRightGame` (`self.LeftRight`)
    (:`NewEnumerator0`
      (`SceneComponent.SetRelativeScale3D` _flipbook (-6.0 6.0 6.7)))
    (:`NewEnumerator1`
      (`SceneComponent.SetRelativeScale3D` _flipbook (6.0 6.0 6.7)))))

(fn `MoveFunction`
  (params (Movement :type "Float (double-precision)"))
  (if (> Movement 0.0)
    (set `self.LeftRight` "NewEnumerator1")
    (`self.FlipFunction` :!label _label)
    (`self.AddMovementInput` (0.35 0.0 0.0) Movement true)
    (elif (< Movement 0.0)
      (set `self.LeftRight` "NewEnumerator0")
      (goto _label))))

(fn `StopRN`
  (`MovementComponent.StopMovementImmediately` (`self.CharacterMovement`)))

(fn `UserConstructionScript`)