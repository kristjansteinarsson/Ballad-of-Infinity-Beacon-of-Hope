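; Player controller for the 2D character that finds and possesses BP_Player2d_1 on BeginPlay and adds the InputMap2D Enhanced Input context.
; Input actions drive walk, jump, run, dodge roll and attack on that character, slowing walk input while attacking.
; Disabled movement blocks walk, jump and dodge, but not attack or run.
; Attack and grounded dodge are gated by recharge counters, refilled by self-calling Delay events.
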(event `RechargeAttack`
  (if (< (`self.AttackRecharge`) (`self.AttackCooldown`))
    (`KismetSystemLibrary.Delay` 0.02)
    (set `self.AttackRecharge` (+ (`self.AttackRecharge`) 0.1))
    (`self.RechargeAttack`)))

(event `self.ReceiveBeginPlay`
  (`|ExecutionSequence`
    (:`then_0`
      (`EnhancedInputSubsystemInterface.AddMappingContext` (pcsubsystem `EnhancedInputLocalPlayerSubsystem` (`GameplayStatics.GetPlayerController` 0)) "/Game/Blueprint/Character/Controller/InputMap2D.InputMap2D" 0 (struct)))
    (:`then_1`
      (bind _returnvalue (`GameplayStatics.GetActorOfClass` "/Game/Blueprint/Character/BP_Player2d_1.BP_Player2d_1_C"))
      (bind _output_get (set `self.PlayerCharacter` _returnvalue))
      (`self.Possess` _output_get)
      (set `/Game/Blueprint/Character/BP_Player2d_1.PlayerController` self _output_get))))

(event `RechargeDodge`
  (if (< (`self.DodgeRollRecharge`) (`self.DodgeRollCooldown`))
    (`KismetSystemLibrary.Delay` 0.1)
    (set `self.DodgeRollRecharge` (+ (`self.DodgeRollRecharge`) 0.1))
    (`self.RechargeDodge`)))

(event `EnhancedInput|/Game/Blueprint/Character/Controller/IA_Walk`
  (params (ActionValue :type "Float (double-precision)") (ElapsedSeconds :type "Float (double-precision)") (TriggeredSeconds :type "Float (double-precision)") (InputAction :type "InputAction Object Reference" :default "/Game/Blueprint/Character/Controller/IA_Walk.IA_Walk"))
  (bind _playercharacter (`self.PlayerCharacter`))
  (:`Triggered`
    (if (`self.IsMovementDisabled`)
      _
      (elif (`self.IsCharacterAttacking`)
        (`/Game/Blueprint/Character/BP_Player2d_1.MoveFunction` _playercharacter (* ActionValue 0.1))
        (else
          (`/Game/Blueprint/Character/BP_Player2d_1.MoveFunction` _playercharacter ActionValue))))))

(event `EnhancedInput|/Game/Blueprint/Character/Controller/IA_Jump`
  (params (ActionValue :type Boolean) (ElapsedSeconds :type "Float (double-precision)") (TriggeredSeconds :type "Float (double-precision)") (InputAction :type "InputAction Object Reference" :default "/Game/Blueprint/Character/Controller/IA_Jump.IA_Jump"))
  (bind _playercharacter (`self.PlayerCharacter`))
  (:`Triggered`
    (if (not (`self.IsMovementDisabled`))
      (`Character.Jump` _playercharacter)))
  (:`Completed`
    (`Character.StopJumping` _playercharacter)))

(event `EnhancedInput|/Game/Blueprint/Character/Controller/IA_Dodge`
  (params (ActionValue :type Boolean) (ElapsedSeconds :type "Float (double-precision)") (TriggeredSeconds :type "Float (double-precision)") (InputAction :type "InputAction Object Reference" :default "/Game/Blueprint/Character/Controller/IA_Dodge.IA_Dodge"))
  (bind _playercharacter (`self.PlayerCharacter`))
  (:`Triggered`
    (if (and (`NavMovementComponent.IsMovingOnGround` (`Character.CharacterMovement` _playercharacter)) (>= (`self.DodgeRollRecharge`) (`self.DodgeRollCooldown`)) (not (`self.IsMovementDisabled`)))
      (set `self.DodgeRollRecharge` 0.0)
      (`/Game/Blueprint/Character/BP_Player2d_1.DodgeRoll` _playercharacter)
      (`self.RechargeDodge`))))

(event `EnhancedInput|/Game/Blueprint/Character/Controller/IA_AttackR1`
  (params (ActionValue :type Boolean) (ElapsedSeconds :type "Float (double-precision)") (TriggeredSeconds :type "Float (double-precision)") (InputAction :type "InputAction Object Reference" :default "/Game/Blueprint/Character/Controller/IA_AttackR1.IA_AttackR1"))
  (:`Started`
    (if (>= (`self.AttackRecharge`) (`self.AttackCooldown`))
      (`/Game/Blueprint/Character/BP_Player2d_1.Attack` (`self.PlayerCharacter`))
      (set `self.AttackRecharge` 0.0)
      (`self.RechargeAttack`))))

(event `EnhancedInput|/Game/Blueprint/Character/Controller/IA_Run`
  (params (ActionValue :type Boolean) (ElapsedSeconds :type "Float (double-precision)") (TriggeredSeconds :type "Float (double-precision)") (InputAction :type "InputAction Object Reference" :default "/Game/Blueprint/Character/Controller/IA_Run.IA_Run"))
  (bind _playercharacter (`self.PlayerCharacter`))
  (bind _playercharacter_2 (`self.PlayerCharacter`))
  (:`Started`
    (set `/Game/Blueprint/Character/BP_Player2d_1.IsRunning` true _playercharacter_2)
    (set `CharacterMovementComponent.MaxWalkSpeed` 1700.0 (`Character.CharacterMovement` _playercharacter_2))
    (`KismetSystemLibrary.PrintString` "running"))
  (:`Completed`
    (set `/Game/Blueprint/Character/BP_Player2d_1.IsRunning` false _playercharacter)
    (set `CharacterMovementComponent.MaxWalkSpeed` 850.0 (`Character.CharacterMovement` _playercharacter))
    (`KismetSystemLibrary.PrintString` "walking")))

(fn `UserConstructionScript`)