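; Base enemy for a 2D game that feeds its AI controller's Blackboard and handles its own damage and attack.
; BeginPlay seeds home, two patrol points offset along X and attack range.
; Detection and AttackDetection overlaps set the player target and in-range flag, while Hurtbox applies light-attack damage and destroys the enemy at zero health.
; Attack spawns, generates and attaches an attack actor; the Hitbox overlap only casts to the player.
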(event `SetupRange`
  (`BlackboardComponent.SetValueAsFloat` (`AIController.Blackboard` (`self.As AIController`)) "DistanceFromTarget" (`self.Range of attack`)))

(event `SetupHome`
  (bind _output_get (set `self.Home` (`self.K2_GetActorLocation`)))
  (`BlackboardComponent.SetValueAsVector` (`AIController.Blackboard` (`self.As AIController`)) "Home" _output_get))

(event `SetupPatroll`
  (`|ExecutionSequence`
    (:`then_0`
      (`BlackboardComponent.SetValueAsVector` (`AIController.Blackboard` (`self.As AIController`)) "Patrol1" (+ (`self.Home`) (100.0 0.0 0.0))))
    (:`then_1`
      (`BlackboardComponent.SetValueAsVector` (`AIController.Blackboard` (`self.As AIController`)) "Patrol2" (- (`self.Home`) (100.0 0.0 0.0))))))

(event `self.ReceiveBeginPlay`
  (bind _asaicontroller (cast `AIController` (`self.GetController`)))
  (set `self.As AIController` _asaicontroller)
  (`self.SetupHome`)
  (`self.SetupPatroll`)
  (`self.SetupRange`))

(event `self.Hurtbox.OnComponentBeginOverlap`
  (params (OverlappedComponent :type "PrimitiveComponent Object Reference") (OtherActor :type "Actor Object Reference") (OtherComp :type "PrimitiveComponent Object Reference") (OtherBodyIndex :type Integer) (bFromSweep :type Boolean) (SweepResult :type "HitResult Structure (by ref)"))
  (bind _bp_health (`self.BP_Health`))
  (bind _asbp_attack_light_1 (cast `/Game/Blueprint/Character/Attacks/Melee/BP_Attack_Light_1` OtherActor))
  (`/Game/Blueprint/Components/BP_Health.TakeDamage` _bp_health (`/Game/Blueprint/Character/Attacks/Melee/BP_Attack_Light_1.Damage` _asbp_attack_light_1))
  (if (not (> (`/Game/Blueprint/Components/BP_Health.Health` _bp_health) 0.0))
    (`self.K2_DestroyActor`)))

(event `self.Detection.OnComponentBeginOverlap`
  (params (OverlappedComponent :type "PrimitiveComponent Object Reference") (OtherActor :type "Actor Object Reference") (OtherComp :type "PrimitiveComponent Object Reference") (OtherBodyIndex :type Integer) (bFromSweep :type Boolean) (SweepResult :type "HitResult Structure (by ref)"))
  (bind _asbp_player_2d_1 (cast `/Game/Blueprint/Character/BP_Player2d_1` OtherActor))
  (`BlackboardComponent.SetValueAsObject` (`AIController.Blackboard` (`self.As AIController`)) "Target" _asbp_player_2d_1))

(event `self.Detection.OnComponentEndOverlap`
  (params (OverlappedComponent :type "PrimitiveComponent Object Reference") (OtherActor :type "Actor Object Reference") (OtherComp :type "PrimitiveComponent Object Reference") (OtherBodyIndex :type Integer))
  (cast `/Game/Blueprint/Character/BP_Player2d_1` OtherActor)
  (`BlackboardComponent.SetValueAsObject` (`AIController.Blackboard` (`self.As AIController`)) "Target" null))

(event `self.AttackDetection.OnComponentBeginOverlap`
  (params (OverlappedComponent :type "PrimitiveComponent Object Reference") (OtherActor :type "Actor Object Reference") (OtherComp :type "PrimitiveComponent Object Reference") (OtherBodyIndex :type Integer) (bFromSweep :type Boolean) (SweepResult :type "HitResult Structure (by ref)"))
  (cast `/Game/Blueprint/Character/BP_Player2d_1` OtherActor)
  (`BlackboardComponent.SetValueAsBool` (`AIController.Blackboard` (`self.As AIController`)) "IsEnemyInRange" true))

(event `self.AttackDetection.OnComponentEndOverlap`
  (params (OverlappedComponent :type "PrimitiveComponent Object Reference") (OtherActor :type "Actor Object Reference") (OtherComp :type "PrimitiveComponent Object Reference") (OtherBodyIndex :type Integer))
  (cast `/Game/Blueprint/Character/BP_Player2d_1` OtherActor)
  (`BlackboardComponent.SetValueAsBool` (`AIController.Blackboard` (`self.As AIController`)) "IsEnemyInRange" false))

(event `self.Hitbox.OnComponentBeginOverlap`
  (params (OverlappedComponent :type "PrimitiveComponent Object Reference") (OtherActor :type "Actor Object Reference") (OtherComp :type "PrimitiveComponent Object Reference") (OtherBodyIndex :type Integer) (bFromSweep :type Boolean) (SweepResult :type "HitResult Structure (by ref)"))
  (cast `/Game/Blueprint/Character/BP_Player2d_1` OtherActor))

(fn `Attack`
  (bind _returnvalue (`|SpawnActorFromClass` "/Game/Blueprint/Enemies/BaseEnemyAttack.BaseEnemyAttack_C" (`KismetMathLibrary.MakeTransform` (160.0 0.0 0.0) (`self.K2_GetActorRotation` self) (`KismetMathLibrary.MakeVector` (.x (`SceneComponent.RelativeScale3D` (`self.Sprite`))) (.y (`SceneComponent.RelativeScale3D` (`self.Sprite`))) (.z (`SceneComponent.RelativeScale3D` (`self.Sprite`))))) "Undefined" "MultiplyWithRoot" null null))
  (`/Game/Blueprint/Enemies/BaseEnemyAttack.Generate` _returnvalue)
  (`self.K2_AttachToActor` _returnvalue self "None" "KeepRelative" "KeepWorld" "KeepRelative" true))

(fn `UserConstructionScript`)