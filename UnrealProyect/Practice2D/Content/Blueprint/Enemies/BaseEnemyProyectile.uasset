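; Base enemy projectile for a 2D game that damages the player on contact.
; The construction script feeds Speed into the projectile movement component as both initial and max speed.
; On overlap with BP_Player2d_1 it applies Damage through that player's BPHealth component and does not destroy itself.
; A Generate event applies the configured Sprite to its Paper2D sprite component.
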(event `self.ReceiveActorBeginOverlap`
  (params (OtherActor :type "Actor Object Reference"))
  (bind _asbp_player_2d_1 (cast `/Game/Blueprint/Character/BP_Player2d_1` OtherActor))
  (`/Game/Blueprint/Components/BP_Health.TakeDamage` (`/Game/Blueprint/Character/BP_Player2d_1.BP_Health` _asbp_player_2d_1) (`self.Damage`)))

(event `self.Generate`
  (`PaperSpriteComponent.SetSprite` (`self.PaperSprite`) (`self.Sprite`)))

(fn `UserConstructionScript`
  (bind _projectilemovement (`self.ProjectileMovement`))
  (bind _speed (`self.Speed`))
  (`parent.UserConstructionScript`)
  (set `ProjectileMovementComponent.MaxSpeed` _speed _projectilemovement)
  (set `ProjectileMovementComponent.InitialSpeed` _speed _projectilemovement))