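; Behavior tree task for enemies that computes an attack position beside the current target.
; It reads the Target actor and DistanceFromTarget from the blackboard, then offsets the target's location along X toward whichever side the pawn is on.
; The result is stored in the NewPositiontoattack key and the task finishes successfully; it does not move the pawn itself.
; A failed Target cast stops execution without calling FinishExecute.
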(event `self.ReceiveExecuteAI`
  (params (OwnerController :type "AIController Object Reference") (ControlledPawn :type "Pawn Object Reference"))
  (bind _returnvalue (`AIBlueprintHelperLibrary.GetBlackboard` ControlledPawn))
  (bind _returnvalue_2 (`BlackboardComponent.GetValueAsFloat` _returnvalue "DistanceFromTarget"))
  (bind _asactor (cast `Actor` (`BlackboardComponent.GetValueAsObject` _returnvalue "Target")))
  (bind _x (.x (.location (`Actor.GetTransform` _asactor))))
  (bind _y (.y (.location (`Actor.GetTransform` _asactor))))
  (bind _z (.z (.location (`Actor.GetTransform` _asactor))))
  (if (> (.x (.location (`Actor.GetTransform` ControlledPawn))) _x)
    (`BlackboardComponent.SetValueAsVector` _returnvalue "NewPositiontoattack" (`KismetMathLibrary.MakeVector` (+ _x _returnvalue_2) _y _z))
    (else
      (`BlackboardComponent.SetValueAsVector` _returnvalue "NewPositiontoattack" (`KismetMathLibrary.MakeVector` (- _x _returnvalue_2) _y _z))))
  (`self.FinishExecute` true))