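; Crawler enemy Blueprint that supplies a ranged attack by firing a projectile.
; Attack spawns a BaseEnemyProyectile with a set speed, using the actor's rotation and the sprite's relative scale.
; The spawn location is a fixed vector, not offset from the actor's position.
; The event graph holds only disabled placeholder events, and the construction script just calls its parent.
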(fn `Attack`
  (`|SpawnActorFromClass` "/Game/Blueprint/Enemies/BaseEnemyProyectile.BaseEnemyProyectile_C" (`KismetMathLibrary.MakeTransform` (160.0 0.0 0.0) (`self.K2_GetActorRotation` self) (`KismetMathLibrary.MakeVector` (.x (`SceneComponent.RelativeScale3D` (`self.Sprite`))) (.y (`SceneComponent.RelativeScale3D` (`self.Sprite`))) (.z (`SceneComponent.RelativeScale3D` (`self.Sprite`))))) "Undefined" "MultiplyWithRoot" null 300.0 null))

(fn `UserConstructionScript`
  (`parent.UserConstructionScript`))