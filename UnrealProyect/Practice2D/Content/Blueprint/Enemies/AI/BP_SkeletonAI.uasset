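; BP_SkeletonAI is the skeleton enemy's AI controller, running BT_Skeleton when it possesses its pawn.
; AI Perception updates that sense a Player-tagged actor cancel the timer and write the target and line-of-sight flag to the blackboard.
; Any other perception update starts a LineOfSightTime timer that clears both keys on expiry, giving a grace period before the target is forgotten.
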(event `self.ReceivePossess`
  (params (PossessedPawn :type "Pawn Object Reference"))
  (`self.RunBehaviorTree` "/Game/Blueprint/Enemies/AI/BT_Skeleton.BT_Skeleton"))

(event `self.AIPerception.OnTargetPerceptionUpdated`
  (params (Actor :type "Actor Object Reference") (Stimulus :type "AIStimulus Structure"))
  (bind _returnvalue (`AIBlueprintHelperLibrary.GetBlackboard` null))
  (if (and (`self.ActorHasTag` Actor "Player") (`.bSuccessfullySensed` (break `AIStimulus` Stimulus)))
    (`KismetSystemLibrary.K2_ClearAndInvalidateTimerHandle` (`self.EnemyTimer`))
    (`BlackboardComponent.SetValueAsBool` _returnvalue (`self.HasLineOfSight`) true)
    (`BlackboardComponent.SetValueAsObject` _returnvalue (`self.EnemyActor`) Actor)
    (else
      (bind _returnvalue_2 (`KismetSystemLibrary.K2_SetTimerDelegate` (delegate `StartEnemyTimer`) (`self.LineOfSightTime`)))
      (set `self.EnemyTimer` _returnvalue_2))))

(event `StartEnemyTimer`
  (bind _returnvalue (`AIBlueprintHelperLibrary.GetBlackboard` null))
  (`BlackboardComponent.SetValueAsBool` _returnvalue (`self.HasLineOfSight`) false)
  (`BlackboardComponent.SetValueAsObject` _returnvalue (`self.EnemyActor`) null))

(fn `UserConstructionScript`)