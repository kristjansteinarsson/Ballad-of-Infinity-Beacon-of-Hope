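; BP_Health is a health component that applies typed damage to a Health value.
; TakeDamage subtracts Defense from each damage type (physical, elemental and others), scales it by that type's Resistance multiplier, and sums the results with Unblockeable damage, which bypasses both.
; It subtracts the total from Health and returns the new value, with no clamping, so Defense above Damage can produce healing.
; The event graph holds no active logic.
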(fn `TakeDamage`
  (params (Damage :type "/Game/Blueprint/Components/Str_Damage Structure"))
  (returns (TakenDamage :type "Float (double-precision)"))
  (bind (_slash _pierce _blunt _fire _ice _entropic _acid _radiant _crushing _unblockeable) (break `/Game/Blueprint/Components/Str_Damage` Damage))
  (bind (_slash_2 _pierce_2 _blunt_2 _fire_2 _ice_2 _entropic_2 _acid_2 _radiant_2 _crushing_2) (break `/Game/Blueprint/Components/Str_Damage` (`self.Defense`)))
  (bind (_slash_3 _pierce_3 _blunt_3 _fire_3 _ice_3 _entropic_3 _acid_3 _radiant_3 _crushing_3) (break `/Game/Blueprint/Components/Str_Damage` (`self.Resistance`)))
  (bind _output_get (set `self.Health` (- (`self.Health`) (+ (* (- _slash _slash_2) _slash_3) (* (- _pierce _pierce_2) _pierce_3) (* (- _blunt _blunt_2) _blunt_3) (* (- _fire _fire_2) _fire_3) (* (- _ice _ice_2) _ice_3) (* (- _entropic _entropic_2) _entropic_3) (* (- _acid _acid_2) _acid_3) (* (- _radiant _radiant_2) _radiant_3) (* (- _crushing _crushing_2) _crushing_3) _unblockeable))))
  (return _output_get))