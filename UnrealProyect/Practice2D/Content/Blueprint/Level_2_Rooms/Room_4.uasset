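; Level 2 Room 4 is an arena encounter that locks the 2D player in until its enemies are destroyed.
; A one-shot trigger box turns on two blocking walls, briefly shows four vents and spawns a BP_BaseEnemy at each.
; Tick repeatedly binds the enemies' OnDestroyed events through nested validity checks.
; The handler counts kills and, after the fourth, waits briefly before hiding and disabling the walls.
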(event `OnDestroyed_Event`
  (params (DestroyedActor :type "Actor Object Reference"))
  (bind _block1 (`self.Block1`))
  (bind _kills (`self.Kills`))
  (set `self.Kills` (+ _kills 1))
  (if (>= _kills 4)
    (`KismetSystemLibrary.Delay` 2.0)
    (`PrimitiveComponent.SetCollisionEnabled` _block1 "NoCollision")
    (`PrimitiveComponent.SetCollisionEnabled` (`self.Block2`) "NoCollision")
    (`SceneComponent.SetVisibility` _block1 false false)
    (`SceneComponent.SetVisibility` (`self.Block2`) false false)))

(event `self.ReceiveTick`
  (params (DeltaSeconds :type "Float (single-precision)"))
  (`/Engine/EditorBlueprintResources/StandardMacros.IsValid` (stale `self.Box.OnComponentBeginOverlap` _returnvalue)
    (:`Is Valid`
      (add `self.OnDestroyed` (stale `self.Box.OnComponentBeginOverlap` _returnvalue) (delegate `OnDestroyed_Event`))
      (`/Engine/EditorBlueprintResources/StandardMacros.IsValid` (stale `self.Box.OnComponentBeginOverlap` _returnvalue_2)
        (:`Is Valid`
          (add `self.OnDestroyed` (stale `self.Box.OnComponentBeginOverlap` _returnvalue_2) (delegate `OnDestroyed_Event`))
          (`/Engine/EditorBlueprintResources/StandardMacros.IsValid` (stale `self.Box.OnComponentBeginOverlap` _returnvalue_3)
            (:`Is Valid`
              (add `self.OnDestroyed` (stale `self.Box.OnComponentBeginOverlap` _returnvalue_3) (delegate `OnDestroyed_Event`))
              (`/Engine/EditorBlueprintResources/StandardMacros.IsValid` (stale `self.Box.OnComponentBeginOverlap` _returnvalue_4)
                (:`Is Valid`
                  (add `self.OnDestroyed` (stale `self.Box.OnComponentBeginOverlap` _returnvalue_4) (delegate `OnDestroyed_Event`)))))))))))

(event `self.ReceiveBeginPlay`
  (`PrimitiveComponent.SetCollisionEnabled` (`self.Block1`) "NoCollision")
  (`PrimitiveComponent.SetCollisionEnabled` (`self.Block2`) "NoCollision")
  (`PrimitiveComponent.SetCollisionEnabled` (`self.VentTop1`) "NoCollision")
  (`PrimitiveComponent.SetCollisionEnabled` (`self.VentTop2`) "NoCollision")
  (`PrimitiveComponent.SetCollisionEnabled` (`self.VentTop3`) "NoCollision")
  (`PrimitiveComponent.SetCollisionEnabled` (`self.VentTop4`) "NoCollision")
  (`PrimitiveComponent.SetCollisionEnabled` (`self.Vent1`) "NoCollision")
  (`PrimitiveComponent.SetCollisionEnabled` (`self.Vent2`) "NoCollision")
  (`PrimitiveComponent.SetCollisionEnabled` (`self.Vent4`) "NoCollision")
  (`PrimitiveComponent.SetCollisionEnabled` (`self.Vent3`) "NoCollision")
  (`SceneComponent.SetVisibility` (`self.Vent4`) false false)
  (`SceneComponent.SetVisibility` (`self.Vent3`) false false)
  (`SceneComponent.SetVisibility` (`self.Vent2`) false false)
  (`SceneComponent.SetVisibility` (`self.Vent1`) false false)
  (`SceneComponent.SetVisibility` (`self.Block1`) false false)
  (`SceneComponent.SetVisibility` (`self.Block2`) false false))

(event `self.Box.OnComponentBeginOverlap`
  (params (OverlappedComponent :type "PrimitiveComponent Object Reference") (OtherActor :type "Actor Object Reference") (OtherComp :type "PrimitiveComponent Object Reference") (OtherBodyIndex :type Integer) (bFromSweep :type Boolean) (SweepResult :type "HitResult Structure (by ref)"))
  (bind _block1 (`self.Block1`))
  (cast `/Game/Blueprint/Character/BP_Player2d_1` OtherActor)
  (`ActorComponent.K2_DestroyComponent` (`self.Box`))
  (`PrimitiveComponent.SetCollisionEnabled` _block1 "QueryAndPhysics")
  (`PrimitiveComponent.SetCollisionEnabled` (`self.Block2`) "QueryAndPhysics")
  (`SceneComponent.SetVisibility` _block1 true false)
  (`SceneComponent.SetVisibility` (`self.Block2`) true false)
  (`SceneComponent.SetVisibility` (`self.Vent1`) true false)
  (`SceneComponent.SetVisibility` (`self.Vent2`) true false)
  (`SceneComponent.SetVisibility` (`self.Vent3`) true false)
  (`SceneComponent.SetVisibility` (`self.Vent4`) true false)
  (`KismetSystemLibrary.Delay` 0.2)
  (bind _returnvalue (`|SpawnActorFromClass` "/Game/Blueprint/Enemies/BP_BaseEnemy.BP_BaseEnemy_C" (`KismetMathLibrary.MakeTransform` (`SceneComponent.K2_GetComponentLocation` (`self.Vent1`))) "Undefined" "MultiplyWithRoot" null null))
  (bind _returnvalue_2 (`|SpawnActorFromClass` "/Game/Blueprint/Enemies/BP_BaseEnemy.BP_BaseEnemy_C" (`KismetMathLibrary.MakeTransform` (`SceneComponent.K2_GetComponentLocation` (`self.Vent2`))) "Undefined" "MultiplyWithRoot" null null))
  (bind _returnvalue_3 (`|SpawnActorFromClass` "/Game/Blueprint/Enemies/BP_BaseEnemy.BP_BaseEnemy_C" (`KismetMathLibrary.MakeTransform` (`SceneComponent.K2_GetComponentLocation` (`self.Vent3`))) "Undefined" "MultiplyWithRoot" null null))
  (bind _returnvalue_4 (`|SpawnActorFromClass` "/Game/Blueprint/Enemies/BP_BaseEnemy.BP_BaseEnemy_C" (`KismetMathLibrary.MakeTransform` (`SceneComponent.K2_GetComponentLocation` (`self.Vent4`))) "Undefined" "MultiplyWithRoot" null null))
  (`KismetSystemLibrary.Delay` 0.4)
  (`SceneComponent.SetVisibility` (`self.Vent1`) false false)
  (`SceneComponent.SetVisibility` (`self.Vent2`) false false)
  (`SceneComponent.SetVisibility` (`self.Vent3`) false false)
  (`SceneComponent.SetVisibility` (`self.Vent4`) false false))

(fn `UserConstructionScript`)