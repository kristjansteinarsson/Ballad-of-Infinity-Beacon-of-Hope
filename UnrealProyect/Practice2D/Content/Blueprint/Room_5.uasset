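; Boss room Blueprint that plays a one-shot intro cutscene when the 2D player enters its trigger box.
; Overlap destroys the trigger, disables input and starts boss audio, which hands off to a second track when finished.
; Timelines pan the player's spring arm out and back around two sequential boss moves to marker positions.
; Afterwards it shows a widget, restores input and enables the initially hidden Cube with collision.
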(event `OnAudioFinished_Event`
  (`GameplayStatics.SpawnSound2D` "/Game/Music/Boss2-Wrap.Boss2-Wrap" 1.0 1.0 0.0 null false false))

(event `self.ReceiveBeginPlay`
  (`SceneComponent.SetVisibility` (`self.BossPosition`) false false)
  (`SceneComponent.SetVisibility` (`self.BossPosition1`) false false)
  (`SceneComponent.SetVisibility` (`self.Cube`) false false)
  (`PrimitiveComponent.SetCollisionEnabled` (`self.Cube`) "NoCollision"))

(event `self.Box.OnComponentBeginOverlap`
  (params (OverlappedComponent :type "PrimitiveComponent Object Reference") (OtherActor :type "Actor Object Reference") (OtherComp :type "PrimitiveComponent Object Reference") (OtherBodyIndex :type Integer) (bFromSweep :type Boolean) (SweepResult :type "HitResult Structure (by ref)"))
  (bind _boss (`self.Boss`))
  (bind _cube (`self.Cube`))
  (bind _relativerotation (`SceneComponent.RelativeRotation` _boss))
  (bind _asbp_player_2d_1 (cast `/Game/Blueprint/Character/BP_Player2d_1` OtherActor))
  (`ActorComponent.K2_DestroyComponent` (`self.Box`))
  (bind _playercontroller (`/Game/Blueprint/Character/BP_Player2d_1.PlayerController` _asbp_player_2d_1))
  (`self.DisableInput` _playercontroller _playercontroller)
  (bind _returnvalue (`GameplayStatics.SpawnSound2D` "/Game/Music/Boss1.Boss1" 1.0 1.0 0.0 null))
  (add `AudioComponent.OnAudioFinished` _returnvalue (delegate `OnAudioFinished_Event`))
  (bind (_direction _alpha) (`Timeline|Timeline` :!via `PlayFromStart`)
    (:`Update`
      (bind _springarm (`/Game/Blueprint/Character/BP_Player2d_1.SpringArm` _asbp_player_2d_1))
      (bind _returnvalue_2 (* (* _alpha 15.0) 1.5))
      (`SceneComponent.K2_SetRelativeLocation` _springarm (+ (`SceneComponent.RelativeLocation` _springarm) (`KismetMathLibrary.MakeVector` _returnvalue_2 _returnvalue_2)) false false))
    (:`Finished`
      (`KismetSystemLibrary.MoveComponentTo` _boss (`SceneComponent.RelativeLocation` (`self.BossPosition`)) _relativerotation true true 5.5)
      (`KismetSystemLibrary.MoveComponentTo` _boss (`SceneComponent.RelativeLocation` (`self.BossPosition1`)) _relativerotation true true 4.0)
      (bind (_direction_2 _alpha_2) (`Timeline|Timeline_0` :!via `PlayFromStart`)
        (:`Update`
          (bind _springarm_2 (`/Game/Blueprint/Character/BP_Player2d_1.SpringArm` _asbp_player_2d_1))
          (bind _returnvalue_3 (* (* _alpha_2 -15.0) -1.5))
          (`SceneComponent.K2_SetRelativeLocation` _springarm_2 (- (`SceneComponent.RelativeLocation` _springarm_2) (`KismetMathLibrary.MakeVector` _returnvalue_3 _returnvalue_3)) false false))
        (:`Finished`
          (`KismetSystemLibrary.Delay` 1.0)
          (bind _returnvalue_4 (`|CreateWidget` "/Game/Blueprint/Widgets/W_Main1.W_Main1_C"))
          (`UserWidget.AddToViewport` _returnvalue_4 0)
          (`self.EnableInput` _playercontroller _playercontroller)
          (`SceneComponent.SetVisibility` _cube true false)
          (`PrimitiveComponent.SetCollisionEnabled` _cube "QueryAndPhysics"))))))

(fn `UserConstructionScript`)