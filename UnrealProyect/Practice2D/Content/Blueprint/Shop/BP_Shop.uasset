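; BP_Shop is a shop actor that sells the player three upgrades: a weapon, armor defense and roll i-frames.
; Overlapping its sphere stores the BP_Player2d_1 reference and enables input on the shop; nothing disables it afterwards.
; Up and down inputs cycle the selection with wraparound, reported only through debug prints.
; Enter reads the selected item's cost from the Stuff data table, deducts coins if affordable and sets that upgrade directly on the player.
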(event `self.Sphere.OnComponentBeginOverlap`
  (params (OverlappedComponent :type "PrimitiveComponent Object Reference") (OtherActor :type "Actor Object Reference") (OtherComp :type "PrimitiveComponent Object Reference") (OtherBodyIndex :type Integer) (bFromSweep :type Boolean) (SweepResult :type "HitResult Structure (by ref)"))
  (bind _asbp_player_2d_1 (cast `/Game/Blueprint/Character/BP_Player2d_1` OtherActor))
  (set `self.As BP Player 2d 1` _asbp_player_2d_1)
  (`self.EnableInput` (`/Game/Blueprint/Character/BP_Player2d_1.PlayerController` _asbp_player_2d_1)))

(event `EnhancedInput|/Game/Blueprint/Character/Controller/IA_SelectUP`
  (params (ActionValue :type Boolean) (ElapsedSeconds :type "Float (double-precision)") (TriggeredSeconds :type "Float (double-precision)") (InputAction :type "InputAction Object Reference" :default "/Game/Blueprint/Character/Controller/IA_SelectUP.IA_SelectUP"))
  (:`Started`
    (bind _output_get (set `self.Current item` (- (`self.Current item`) 1)))
    (if (<= _output_get -1)
      (set `self.Current item` 2))
    (`KismetSystemLibrary.PrintString` (`KismetStringLibrary.Conv_IntToString` _output_get))))

(event `EnhancedInput|/Game/Blueprint/Character/Controller/IA_SelectDown`
  (params (ActionValue :type Boolean) (ElapsedSeconds :type "Float (double-precision)") (TriggeredSeconds :type "Float (double-precision)") (InputAction :type "InputAction Object Reference" :default "/Game/Blueprint/Character/Controller/IA_SelectDown.IA_SelectDown"))
  (:`Started`
    (bind _output_get (set `self.Current item` (+ (`self.Current item`) 1)))
    (if (>= _output_get 3)
      (set `self.Current item` 0))
    (`KismetSystemLibrary.PrintString` (`KismetStringLibrary.Conv_IntToString` _output_get))))

(event `EnhancedInput|/Game/Blueprint/Character/Controller/IA_SelectEnter`
  (params (ActionValue :type Boolean) (ElapsedSeconds :type "Float (double-precision)") (TriggeredSeconds :type "Float (double-precision)") (InputAction :type "InputAction Object Reference" :default "/Game/Blueprint/Character/Controller/IA_SelectEnter.IA_SelectEnter"))
  (bind _stuff (`self.Stuff`))
  (bind _as_bp_player_2d_1 (`self.As BP Player 2d 1`))
  (bind (_name _cost) (break `/Game/Blueprint/Shop/Store_Item` (`self.StoreItem`)))
  (bind _currentcoins (`/Game/Blueprint/Character/BP_Player2d_1.CurrentCoins` _as_bp_player_2d_1))
  (:`Started`
    (switch `int` (`self.Current item`)
      (:`0`
        (bind _returnvalue (`|GetDataTableRow` _stuff "0")
          (:`then`
            (set `self.StoreItem` _returnvalue))))
      (:`1`
        (bind _returnvalue_2 (`|GetDataTableRow` _stuff "1")
          (:`then`
            (set `self.StoreItem` _returnvalue_2))))
      (:`2`
        (bind _returnvalue_3 (`|GetDataTableRow` _stuff "2")
          (:`then`
            (set `self.StoreItem` _returnvalue_3)))))
    (if (>= _currentcoins _cost)
      (set `/Game/Blueprint/Character/BP_Player2d_1.CurrentCoins` (- _currentcoins _cost) _as_bp_player_2d_1)
      (switch `int` (`self.Current item`)
        (:`0`
          (set `/Game/Blueprint/Character/BP_Player2d_1.WeaponRightHand` "BettweWeapon" _as_bp_player_2d_1)
          (`KismetSystemLibrary.PrintString` "New weapon"))
        (:`1`
          (set `/Game/Blueprint/Components/BP_Health.Defense` (make `/Game/Blueprint/Components/Str_Damage` 25.0) (`/Game/Blueprint/Character/BP_Player2d_1.BP_Health` _as_bp_player_2d_1))
          (`KismetSystemLibrary.PrintString` "Armor up"))
        (:`2`
          (set `/Game/Blueprint/Character/BP_Player2d_1.RollIFrames` 9 _as_bp_player_2d_1)
          (`KismetSystemLibrary.PrintString` "Rolling stones")))
      (else
        (`KismetSystemLibrary.PrintString` "Fuck no cash")))))

(fn `UserConstructionScript`)