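; Room_4 is a room Blueprint that seals two blockers in place when the player enters its trigger.
; On BeginPlay, Block1 and Block2 are hidden and have no collision.
; When BP_Player2d_1 overlaps the Box, both blocks become visible with query and physics collision, and nothing in the graph turns them off again.
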(event `self.ReceiveBeginPlay`
  (bind _block1 (`self.Block1`))
  (bind _block2 (`self.Block2`))
  (`PrimitiveComponent.SetCollisionEnabled` _block1 "NoCollision")
  (`PrimitiveComponent.SetCollisionEnabled` _block2 "NoCollision")
  (`SceneComponent.SetVisibility` _block1 false false)
  (`SceneComponent.SetVisibility` _block2 false false))

(event `self.Box.OnComponentBeginOverlap`
  (params (OverlappedComponent :type "PrimitiveComponent Object Reference") (OtherActor :type "Actor Object Reference") (OtherComp :type "PrimitiveComponent Object Reference") (OtherBodyIndex :type Integer) (bFromSweep :type Boolean) (SweepResult :type "HitResult Structure (by ref)"))
  (bind _block1 (`self.Block1`))
  (bind _block2 (`self.Block2`))
  (cast `/Game/Blueprint/Character/BP_Player2d_1` OtherActor)
  (`PrimitiveComponent.SetCollisionEnabled` _block1 "QueryAndPhysics")
  (`PrimitiveComponent.SetCollisionEnabled` _block2 "QueryAndPhysics")
  (`SceneComponent.SetVisibility` _block1 true false)
  (`SceneComponent.SetVisibility` _block2 true false))

(fn `UserConstructionScript`)