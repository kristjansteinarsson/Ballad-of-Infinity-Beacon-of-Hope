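; One-way platform that the 2D player can pass up through from below and drop down through from above.
; Overlapping the Below trigger disables the Box's collision until the player leaves it.
; The Above trigger enables input and opens a gate so a negative IA_Down value disables Box collision.
; Leaving Above closes the gate and restores collision after a short delay.
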(event `self.Below.OnComponentBeginOverlap`
  (params (OverlappedComponent :type "PrimitiveComponent Object Reference") (OtherActor :type "Actor Object Reference") (OtherComp :type "PrimitiveComponent Object Reference") (OtherBodyIndex :type Integer) (bFromSweep :type Boolean) (SweepResult :type "HitResult Structure (by ref)"))
  (cast `/Game/Blueprint/Character/BP_Player2d_1` OtherActor)
  (`PrimitiveComponent.SetCollisionEnabled` (`self.Box`) "NoCollision"))

(event `self.Below.OnComponentEndOverlap`
  (params (OverlappedComponent :type "PrimitiveComponent Object Reference") (OtherActor :type "Actor Object Reference") (OtherComp :type "PrimitiveComponent Object Reference") (OtherBodyIndex :type Integer))
  (cast `/Game/Blueprint/Character/BP_Player2d_1` OtherActor)
  (`PrimitiveComponent.SetCollisionEnabled` (`self.Box`) "QueryAndPhysics"))

(event `EnhancedInput|/Game/Blueprint/Character/Controller/IA_Down`
  (params (ActionValue :type "Float (double-precision)") (ElapsedSeconds :type "Float (double-precision)") (TriggeredSeconds :type "Float (double-precision)") (InputAction :type "InputAction Object Reference" :default "/Game/Blueprint/Character/Controller/IA_Down.IA_Down"))
  (:`Triggered`
    (if (< ActionValue 0.0)
      (`/Engine/EditorBlueprintResources/StandardMacros.Gate` true :!label _label
        (:`Exit`
          (`PrimitiveComponent.SetCollisionEnabled` (`self.Box`) "NoCollision"))))))

(event `self.Above.OnComponentBeginOverlap`
  (params (OverlappedComponent :type "PrimitiveComponent Object Reference") (OtherActor :type "Actor Object Reference") (OtherComp :type "PrimitiveComponent Object Reference") (OtherBodyIndex :type Integer) (bFromSweep :type Boolean) (SweepResult :type "HitResult Structure (by ref)"))
  (cast `/Game/Blueprint/Character/BP_Player2d_1` OtherActor)
  (`self.EnableInput` (`GameplayStatics.GetPlayerController` 0))
  (goto _label :!via `Open`))

(event `self.Above.OnComponentEndOverlap`
  (params (OverlappedComponent :type "PrimitiveComponent Object Reference") (OtherActor :type "Actor Object Reference") (OtherComp :type "PrimitiveComponent Object Reference") (OtherBodyIndex :type Integer))
  (cast `/Game/Blueprint/Character/BP_Player2d_1` OtherActor)
  (`|ExecutionSequence`
    (:`then_0`
      (goto _label :!via `Close`))
    (:`then_1`
      (`KismetSystemLibrary.Delay` 0.2)
      (`PrimitiveComponent.SetCollisionEnabled` (`self.Box`) "QueryAndPhysics"))))

(fn `UserConstructionScript`)