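; A 2D fragile floor block that crumbles when the player touches it and later restores itself.
; A hit on the Box or an overlap with the PlayerStanding trigger casts to BP_Player2d_1 and starts one shared timed sequence.
; The sequence swaps to the fragile flipbook, hides the block and disables its collision after a short delay, then restores visibility, collision and the normal flipbook after a longer one.
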(event `self.Box.OnComponentHit`
  (params (HitComponent :type "PrimitiveComponent Object Reference") (OtherActor :type "Actor Object Reference") (OtherComp :type "PrimitiveComponent Object Reference") (NormalImpulse :type "Vector Structure") (Hit :type "HitResult Structure (by ref)"))
  (cast `/Game/Blueprint/Character/BP_Player2d_1` (stale `self.PlayerStanding.OnComponentBeginOverlap` OtherActor) :!label _label)
  (`PaperFlipbookComponent.SetFlipbook` (`self.Flipbook`) "/Game/Craftpix/6_Traps/FB_FragileBlock.FB_FragileBlock")
  (`KismetSystemLibrary.Delay` 1.0)
  (`SceneComponent.SetHiddenInGame` (`self.Flipbook`) true false)
  (`PrimitiveComponent.SetCollisionEnabled` (`self.Box`) "NoCollision")
  (`KismetSystemLibrary.Delay` 5.0)
  (`SceneComponent.SetHiddenInGame` (`self.Flipbook`) false false)
  (`PrimitiveComponent.SetCollisionEnabled` (`self.Box`) "QueryAndPhysics")
  (`PaperFlipbookComponent.SetFlipbook` (`self.Flipbook`) "/Game/Craftpix/6_Traps/FB_Block.FB_Block"))

(event `self.PlayerStanding.OnComponentBeginOverlap`
  (params (OverlappedComponent :type "PrimitiveComponent Object Reference") (OtherActor :type "Actor Object Reference") (OtherComp :type "PrimitiveComponent Object Reference") (OtherBodyIndex :type Integer) (bFromSweep :type Boolean) (SweepResult :type "HitResult Structure (by ref)"))
  (goto _label))

(fn `UserConstructionScript`)