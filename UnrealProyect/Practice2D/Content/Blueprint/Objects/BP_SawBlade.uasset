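; BP_SawBlade is a 2D saw hazard that shuttles between two points and kills the player on contact.
; From BeginPlay, MoveSaw calls itself in an endless loop, pausing, then easing the PaperFlipbook to TargetMovement or TargetMovement2, alternating via the IsMoved flag.
; A Sphere overlap casts the other actor to BP_Player2d_1 and calls its Death.
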(event `MoveSaw`
  (`KismetSystemLibrary.Delay` 1.5)
  (if (`self.IsMoved?`)
    (`KismetSystemLibrary.MoveComponentTo` (`self.PaperFlipbook`) (`SceneComponent.RelativeLocation` (`self.TargetMovement`)) (struct) true true 0.5)
    (set `self.IsMoved?` false)
    (`self.MoveSaw`)
    (else
      (`KismetSystemLibrary.MoveComponentTo` (`self.PaperFlipbook`) (`SceneComponent.RelativeLocation` (`self.TargetMovement2`)) (struct) true true 0.5)
      (set `self.IsMoved?` true)
      (`self.MoveSaw`))))

(event `self.ReceiveBeginPlay`
  (`self.MoveSaw`))

(event `self.Sphere.OnComponentBeginOverlap`
  (params (OverlappedComponent :type "PrimitiveComponent Object Reference") (OtherActor :type "Actor Object Reference") (OtherComp :type "PrimitiveComponent Object Reference") (OtherBodyIndex :type Integer) (bFromSweep :type Boolean) (SweepResult :type "HitResult Structure (by ref)"))
  (bind _asbp_player_2d_1 (cast `/Game/Blueprint/Character/BP_Player2d_1` OtherActor))
  (`/Game/Blueprint/Character/BP_Player2d_1.Death` _asbp_player_2d_1))

(fn `UserConstructionScript`)