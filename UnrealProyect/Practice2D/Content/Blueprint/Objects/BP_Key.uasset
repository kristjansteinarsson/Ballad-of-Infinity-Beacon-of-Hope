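; BP_Key is a key pickup that grants the 2D player a key.
; When its sphere overlaps BP_Player2d_1, it waits briefly, then plays a timeline that shifts the root component along Z, adding a scaled offset on each update.
; When the timeline finishes, the key destroys itself and sets HasKey on the player.
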(event `self.Sphere.OnComponentBeginOverlap`
  (params (OverlappedComponent :type "PrimitiveComponent Object Reference") (OtherActor :type "Actor Object Reference") (OtherComp :type "PrimitiveComponent Object Reference") (OtherBodyIndex :type Integer) (bFromSweep :type Boolean) (SweepResult :type "HitResult Structure (by ref)"))
  (bind _defaultsceneroot (`self.DefaultSceneRoot`))
  (bind _asbp_player_2d_1 (cast `/Game/Blueprint/Character/BP_Player2d_1` OtherActor))
  (`KismetSystemLibrary.Delay` 0.2)
  (bind (_direction _a) (`Timeline|Timeline`)
    (:`Update`
      (`SceneComponent.K2_SetRelativeLocation` _defaultsceneroot (+ (`SceneComponent.RelativeLocation` _defaultsceneroot) (`KismetMathLibrary.MakeVector` 0.0 0.0 (* _a 10.0))) false false))
    (:`Finished`
      (`self.K2_DestroyActor`)
      (set `/Game/Blueprint/Character/BP_Player2d_1.bHasKey` true _asbp_player_2d_1))))

(fn `UserConstructionScript`)