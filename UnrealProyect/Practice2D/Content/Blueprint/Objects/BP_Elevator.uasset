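; BP_Elevator is an elevator that shuttles its static mesh between two scene-component locations when BP_Player2d_1 enters its box trigger.
; The IsOverlapping flag records which end the mesh was sent to, so overlaps alternate the destination of an eased, timed MoveComponentTo.
; A DoOnce guards each direction, and the player leaving the box resets one of them according to that flag.
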(event `self.Box.OnComponentBeginOverlap`
  (params (OverlappedComponent :type "PrimitiveComponent Object Reference") (OtherActor :type "Actor Object Reference") (OtherComp :type "PrimitiveComponent Object Reference") (OtherBodyIndex :type Integer) (bFromSweep :type Boolean) (SweepResult :type "HitResult Structure (by ref)"))
  (bind _staticmesh (`self.StaticMesh`))
  (bind _staticmesh_2 (`self.StaticMesh`))
  (cast `/Game/Blueprint/Character/BP_Player2d_1` OtherActor)
  (if (not (`self.bIsOverlapping`))
    (`/Engine/EditorBlueprintResources/StandardMacros.DoOnce` false :!label _label
      (:`Completed`
        (`KismetSystemLibrary.MoveComponentTo` _staticmesh (`SceneComponent.RelativeLocation` (`self.Scene`)) (`SceneComponent.RelativeRotation` _staticmesh) true true 3.0)
        (set `self.bIsOverlapping` true)))
    (else
      (`/Engine/EditorBlueprintResources/StandardMacros.DoOnce` false :!label _label_2
        (:`Completed`
          (`KismetSystemLibrary.MoveComponentTo` _staticmesh_2 (`SceneComponent.RelativeLocation` (`self.Scene1`)) (`SceneComponent.RelativeRotation` _staticmesh_2) true true 3.0)
          (set `self.bIsOverlapping` false))))))

(event `self.Box.OnComponentEndOverlap`
  (params (OverlappedComponent :type "PrimitiveComponent Object Reference") (OtherActor :type "Actor Object Reference") (OtherComp :type "PrimitiveComponent Object Reference") (OtherBodyIndex :type Integer))
  (cast `/Game/Blueprint/Character/BP_Player2d_1` OtherActor)
  (if (not (`self.bIsOverlapping`))
    (goto _label_2 :!via `Reset`)
    (else
      (goto _label :!via `Reset`))))

(fn `UserConstructionScript`)